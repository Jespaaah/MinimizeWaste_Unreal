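; Player-controlled drone pawn that flies around vacuuming up Trash actors and adds a HUD widget on start.
; Each tick it moves camera-relative with a separate vertical input and eases its yaw toward the camera's.
; While Suck is held, a looping-state flag shows SuckLight and pulls overlapping trash toward the drone.
; Trash in the Killzone no larger than ShipSize is destroyed with a sound, raising TrashPercent.
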(event EventBeginPlay
  (CallFunction|CreateWidget)
  (Components|Animation|PlayAnimation (Variables|Default|GetDrone) "/Game/Models/Drone_Anim_Armature_Fly.Drone_Anim_Armature_Fly" true))

(event EventTick
  (params (DeltaSeconds :type Float%20%28single-precision%29))
  (CallFunction|Move (stale Input|AxisEvents|InputAxisVertical AxisValue) (stale Input|AxisEvents|InputAxisHorizontal AxisValue) (Input|AxisValues|GetUp))
  (|SuckNodes))

(event Input|ActionEvents|InputActionSuck
  (params (Key :type Key%20Structure :default "None"))
  (:Pressed
    (|SuckBool :!label _label))
  (:Released
    (goto _label Released)))

(event Input|AxisEvents|InputAxisHorizontal
  (params (AxisValue :type Float%20%28single-precision%29)))

(event Input|AxisEvents|InputAxisVertical
  (params (AxisValue :type Float%20%28single-precision%29)))

(fn ConstructionScript)

(fn Move
  (params (Vertical :type Float%20%28single-precision%29) (Horizontal :type Float%20%28single-precision%29) (Up :type Float%20%28single-precision%29))
  (bind _returnvalue (Math|Vector|MakeVector Vertical Horizontal 0.0))
  (bind _camera (Variables|Default|GetCamera))
  (bind _returnvalue_2 (Transformation|GetWorldTransform _camera))
  (bind _returnvalue_3 (Math|Transform|TransformDirection _returnvalue_2 _returnvalue))
  (bind (_x _y) (Math|Vector|BreakVector _returnvalue_3))
  ;[1 1 1] Movement
  (Transformation|AddRelativeLocation (Variables|Default|GetDrone) (* (Math|Vector|Normalize (Math|Vector|MakeVector _x _y (* Up (Variables|Default|GetUp/DownSpeed))) 1e-06) (Variables|Default|GetSpeed)) true false)
  (|Rotation))

(fn Suck
  (Rendering|SetVisibility (Variables|Default|GetSuckLight) true false)
  (for _array_element (Collision|GetOverlappingActors (Variables|Default|GetKillzone) "/Game/Blueprints/Trash/Trash.Trash_C" :!class /Script/Engine.PrimitiveComponent)
    (Utilities|CheckTrashSize _array_element))
  (for _array_element_2 (Collision|GetOverlappingActors (Variables|Default|GetSuckLight) "/Game/Blueprints/Trash/Trash.Trash_C" :!class /Script/Engine.PrimitiveComponent)
    (bind _direction (CallFunction|GetSuckDirection _array_element_2))
    (Transformation|AddRelativeLocation (Actor|GetComponentbyClass _array_element_2 "/Script/Engine.PrimitiveComponent") _direction false false)))

(fn GetSuckDirection
  (params (Target :type Actor%20Object%20Reference))
  (return (* (Math|Vector|Normalize (- (Transformation|GetWorldLocation (Variables|Default|GetDrone)) (Transformation|GetActorLocation Target))) (Variables|Default|GetSuckForce))))

(fn CreateWidget
  (bind _returnvalue (UserInterface|CreateWidget "/Game/Widget.Widget_C" (Game|GetPlayerController 0)))
  (UserInterface|Viewport|AddtoViewport _returnvalue 0))

(event Input|AxisEvents|InputAxisMouseHorizontal
  (params (AxisValue :type Float%20%28single-precision%29))
  (Pawn|Input|AddControllerYawInput AxisValue))

(event Input|AxisEvents|InputAxisMouseVertical
  (params (AxisValue :type Float%20%28single-precision%29))
  (Pawn|Input|AddControllerPitchInput AxisValue))